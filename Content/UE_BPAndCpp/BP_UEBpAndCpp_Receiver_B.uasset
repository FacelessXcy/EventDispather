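; Receiver actor in a Blueprint/C++ interop example that listens for a broadcast from the player's sender pawn.
; On BeginPlay it casts player pawn 0 to UEBpAndCpp_Sender and binds a custom event to its UEBpAndCppBroadcast delegate.
; When the delegate fires, the event prints the received parameter on screen in blue.
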(event Custom|UEBpAndCpp_Broadcast_Event
  (params (Param :type Integer))
  (Development|PrintString (Utilities|String|ToString(Integer) Param) true true "(R=0.000000,G=0.000000,B=1.000000,A=1.000000)" 1e+01))

(event EventBeginPlay
  (|CallParentFunction)
  (EventDispatchers|AssignUEBpandCppBroadcast (.AsUEBp%20and%20Cpp%20Sender (Utilities|Casting|CastToUEBpAndCpp_Sender (Game|Player|GetPlayerPawn 0))) (delegate Custom|UEBpAndCpp_Broadcast_Event)))

(event Collision|EventActorBeginOverlap
  (params (OtherActor :type Actor%20Object%20Reference))
  (|CallParentFunction OtherActor) ; This node is disabled and will not be called.\nDrag off pins to build functionality.
)

(event EventTick
  (params (DeltaSeconds :type Float%20%28single-precision%29))
  (|CallParentFunction DeltaSeconds) ; This node is disabled and will not be called.\nDrag off pins to build functionality.
)

(fn ConstructionScript
  (|CallParentFunction))