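; BP_MyBpAndCpp_Sender is a Blueprint event sender that periodically broadcasts a named event carrying random data.
; On BeginPlay it runs the parent logic, then starts a looping timer.
; Each tick of the timer creates a new MyData asset, fills its Param with a random integer and dispatches it as MyBpAndCpp_BPDispatchEvent.
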(event Custom|DoBpDispatchEvent
  (Utilities|FlowControl|Sequence
    (:then_0
      (Variables|Default|SetMyDataRef (.AsMy%20Data (Utilities|Casting|CastToMyData (Class|EventMgr|NewAsset "/Script/EventDispather.MyData")))))
    (:then_1
      (Variables|/Script/EventDispather.MyData|SetParam (Variables|Default|GetMyDataRef) (Math|Random|RandomIntegerinRange 0 100)))
    (:then_2
      (Class|EventMgr|DispatchEvent "MyBpAndCpp_BPDispatchEvent" (Variables|Default|GetMyDataRef)))))

(event EventBeginPlay
  (|CallParentFunction)
  (Utilities|Time|SetTimerbyEvent (delegate Custom|DoBpDispatchEvent) 3.0 true))

(fn ConstructionScript)