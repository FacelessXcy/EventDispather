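; BP_UEBp_Receiver_G is a Blueprint that listens to the UEBpBroadcast event dispatcher on the player pawn, cast to BP_UEbp_Sender.
; On BeginPlay it binds one handler and unbinds it after a five-second delay, while a second Assign-style handler is attached and never removed.
; Each handler prints the broadcast parameter in its own shade of green, contrasting temporary and persistent dispatcher bindings.
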(event Custom|UEBp_Broadcast_Event_0
  (params (Param :type Integer))
  (Development|PrintString (Utilities|String|ToString(Integer) Param) true true "(R=0.413513,G=1.000000,B=0.673445,A=1.000000)" 1e+01))

(event Custom|UEBp_Broadcast_Event
  (params (Param :type Integer))
  (Development|PrintString (Utilities|String|ToString(Integer) Param) true true "(R=0.074001,G=1.000000,B=0.000000,A=1.000000)" 1e+01))

(event EventBeginPlay
  (bind _returnvalue (Game|Player|GetPlayerPawn 0))
  (bind _asbp_uebp_sender (Utilities|Casting|CastToBP_UEbp_Sender _returnvalue))
  (Utilities|FlowControl|Sequence
    (:then_0
      (EventDispatchers|BindEventtoUEBpBroadcast _asbp_uebp_sender (delegate Custom|UEBp_Broadcast_Event))
      (Utilities|FlowControl|Delay 5.0)
      (EventDispatchers|UnbindEventfromUEBpBroadcast _asbp_uebp_sender (delegate Custom|UEBp_Broadcast_Event)))
    (:then_1
      (EventDispatchers|AssignUEBpBroadcast _asbp_uebp_sender (delegate Custom|UEBp_Broadcast_Event_0)))))

(fn ConstructionScript
  (|CallParentFunction))